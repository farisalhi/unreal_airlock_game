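; AI director that paces the alien's pressure on the player through a fear gauge.
; Each Tick builds the clamped gauge from alien proximity and exposure time, flashlight, movement, zoom, health and keycards collected.
; Low fear sends the alien to the player, moderate fear to random points near remaining keycards, otherwise its director target is cleared.
; Keycard locations are cached on BeginPlay and rebuilt on each pickup.
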(event Custom|OnKeycardCollected
  (bind _output_get (Variables|Default|SetKeycardsCollected (+ (Variables|Default|GetKeycardsCollected) 1)))
  (Development|PrintString (Utilities|String|ToString(Integer) _output_get) false false)
  (Development|PrintString "KEYCARD COLLECTED ABOVE" false false)
  (Utilities|Array|Clear (Variables|Default|GetKeycardLocations))
  (bind _outactors (Actor|GetAllActorsOfClass "/Game/AIRLOCK/Blueprints/Player/BP_KeyCard.BP_KeyCard_C"))
  (for _array_element _outactors
    (Utilities|Array|Add (Variables|Default|GetKeycardLocations) (Transformation|GetActorLocation _array_element)))
  (Development|PrintString "KeyCards Locations # BELOW" true true "(R=0.000000,G=0.660000,B=1.000000,A=1.000000)" 1e+01)
  (Development|PrintString (Utilities|String|ToString(Integer) (Utilities|Array|Length (Variables|Default|GetKeycardLocations))) true true "(R=1.000000,G=0.000000,B=0.025776,A=1.000000)" 1e+01))

(event EventBeginPlay
  (bind _outactors (Actor|GetAllActorsOfClass "/Game/AIRLOCK/Blueprints/Player/BP_Player.BP_Player_C"))
  (Variables|Default|SetPlayerReference (Utilities|Array|Get(acopy) _outactors))
  (bind _outactors_2 (Actor|GetAllActorsOfClass "/Game/AIRLOCK/Blueprints/BP_NPC_ALIEN.BP_NPC_ALIEN_C"))
  (Variables|Default|SetAlienReference (Utilities|Array|Get(acopy) _outactors_2))
  (bind _outactors_3 (Actor|GetAllActorsOfClass "/Game/AIRLOCK/Blueprints/Player/BP_KeyCard.BP_KeyCard_C"))
  (for _array_element _outactors_3
    (Utilities|Array|Add (Variables|Default|GetKeycardLocations) (Transformation|GetActorLocation _array_element))))

(event Collision|EventActorBeginOverlap
  (params (OtherActor :type Actor%20Object%20Reference)))

(event EventTick
  (params (DeltaSeconds :type Float%20%28single-precision%29))
  (bind _alienreference (Variables|Default|GetAlienReference))
  (bind _playerreference (Variables|Default|GetPlayerReference))
  (bind _alienreference_2 (Variables|Default|GetAlienReference))
  (bind _playerreference_2 (Variables|Default|GetPlayerReference))
  (if (Utilities|IsValid (Variables|Default|GetPlayerReference))
    (Variables|Default|SetPlayerLocation (Transformation|GetActorLocation (Variables|Default|GetPlayerReference)))
    (Variables|Default|SetAlienLocation (Transformation|GetActorLocation (Variables|Default|GetAlienReference)))
    (bind _output_get (Variables|Default|SetProximityToAlien (Math|Vector|Distance(Vector) (Variables|Default|GetPlayerLocation) (Variables|Default|GetAlienLocation))))
    (if (< _output_get 1.5e+03)
      (Variables|Default|SetTimeSpentNearAlien (+ (Variables|Default|GetTimeSpentNearAlien) DeltaSeconds))
      (else
        (Variables|Default|SetTimeSpentNearAlien (Math|Float|Max(Float) (- (Variables|Default|GetTimeSpentNearAlien) (* DeltaSeconds 2.0)) 0.0))))
    (Variables|Default|SetIsPlayerInDarkness (not (Variables|/Game/AIRLOCK/Blueprints/Player/BP_Player.BP_Player_C|GetFlashlightOn? (Variables|Default|GetPlayerReference))))
    (bind _output_get_2 (Variables|Default|SetFearGauge (Math|Float|Clamp(Float) (+ (+ (+ (Math|Float|SelectFloat -5.0 0.0 (Variables|/Game/AIRLOCK/Blueprints/Player/BP_Player.BP_Player_C|GetIsZooming? _playerreference_2)) (+ (Math|Float|SelectFloat 5.0 0.0 (Variables|/Game/AIRLOCK/Blueprints/Player/BP_Player.BP_Player_C|GetIsCrouching? _playerreference_2)) (Math|Float|SelectFloat -1e+01 1e+01 (Variables|/Game/AIRLOCK/Blueprints/Player/BP_Player.BP_Player_C|GetIsSprinting? _playerreference_2)))) (+ (+ (+ (Math|Float|MapRangeClamped _output_get 0.0 3e+03 5e+01 0.0) (Math|Float|SelectFloat 15.0 0.0 (Variables|Default|GetIsPlayerInDarkness))) (Math|Float|Min(Float) (* (Variables|Default|GetTimeSpentNearAlien) 2.0) 2e+01)) (* (Variables|Default|GetKeycardsCollected) 5))) (Math|Float|MapRangeClamped (Variables|/Game/AIRLOCK/Blueprints/Player/BP_Player.BP_Player_C|GetHealth _playerreference) 0.0 (Variables|/Game/AIRLOCK/Blueprints/Player/BP_Player.BP_Player_C|GetMax%20Health _playerreference) 2e+01 0.0)) 0.0 1e+02)))
    (Development|PrintString (Utilities|String|ToString(Float) _output_get_2) false false)
    (if (Utilities|IsValid (Variables|Default|GetAlienReference))
      (if (< (Variables|Default|GetFearGauge) (Variables|Default|GetLowFearThreshold))
        (Variables|/Game/AIRLOCK/Blueprints/BP_NPC_ALIEN.BP_NPC_ALIEN_C|SetDirectorTargetLocation _alienreference (Variables|Default|GetPlayerLocation))
        (Variables|/Game/AIRLOCK/Blueprints/BP_NPC_ALIEN.BP_NPC_ALIEN_C|SetHasDirectorTarget _alienreference true)
        (Variables|Default|SetCurrentAlienState "GoToPlayerArea")
        (elif (< (Variables|Default|GetFearGauge) (Variables|Default|GetModerateFearThreshold))
          (if (> (Utilities|Array|Length (Variables|Default|GetKeycardLocations)) 0)
            (Variables|/Game/AIRLOCK/Blueprints/BP_NPC_ALIEN.BP_NPC_ALIEN_C|SetDirectorTargetLocation _alienreference_2 (.RandomLocation (AI|Navigation|GetRandomReachablePointinRadius (Utilities|Array|Get(acopy) (Variables|Default|GetKeycardLocations) (Math|Random|RandomIntegerinRange 0 (Utilities|Array|LastIndex (Variables|Default|GetKeycardLocations)))) 6e+02 0 0)))
            (Variables|/Game/AIRLOCK/Blueprints/BP_NPC_ALIEN.BP_NPC_ALIEN_C|SetHasDirectorTarget _alienreference_2 true)
            (Variables|Default|SetCurrentAlienState "PatrolKeycard")
            (else
              (Variables|/Game/AIRLOCK/Blueprints/BP_NPC_ALIEN.BP_NPC_ALIEN_C|SetHasDirectorTarget (Variables|Default|GetAlienReference) false :!label _label)
              (Variables|Default|SetCurrentAlienState "Idle")))
          (else
            (goto _label)))))))

(fn ConstructionScript)

(fn CalculateFearGauge)