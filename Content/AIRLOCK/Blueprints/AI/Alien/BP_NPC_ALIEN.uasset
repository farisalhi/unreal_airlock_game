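; Alien NPC Blueprint that deals repeated contact damage to the player.
; When the player overlaps its capsule, it stores them as the current target, applies damage and plays a hit sound at its own location.
; A looping one-second timer repeats the damage and sound through Deal Contact Damage until the player's end overlap clears it.
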(event OnComponentEndOverlap(Capsule)
  (params (OverlappedComponent :type Primitive%20Component%20Object%20Reference) (OtherActor :type Actor%20Object%20Reference) (OtherComp :type Primitive%20Component%20Object%20Reference) (OtherBodyIndex :type Integer))
  (Utilities|Casting|CastToBP_Player OtherActor)
  (Utilities|Time|ClearandInvalidateTimerbyHandle (Variables|Default|GetDamage%20Timer%20Handle)))

(event OnComponentBeginOverlap(Capsule)
  (params (OverlappedComponent :type Primitive%20Component%20Object%20Reference) (OtherActor :type Actor%20Object%20Reference) (OtherComp :type Primitive%20Component%20Object%20Reference) (OtherBodyIndex :type Integer) (bFromSweep :type Boolean) (SweepResult :type Hit%20Result%20Structure%20%28by%20ref%29))
  (bind _asbp_player (Utilities|Casting|CastToBP_Player OtherActor))
  (Variables|Default|SetCurrent%20Target _asbp_player)
  (Game|Damage|ApplyDamage (Variables|Default|GetCurrent%20Target) 25.0 0 0)
  (Audio|PlaySoundatLocation "/Game/AIRLOCK/Sounds/minecraft_hit_sound___1080p60fps.minecraft_hit_sound___1080p60fps" (Transformation|GetActorLocation) "0, 0, 0" 1.0 1.0 0.0 0 0 0 0)
  (bind _returnvalue (Utilities|Time|SetTimerbyFunctionName 0 "Deal Contact Damage" 1.0 true))
  (Variables|Default|SetDamage%20Timer%20Handle _returnvalue))

(event Custom|Deal%20Contact%20Damage
  (Game|Damage|ApplyDamage (Variables|Default|GetCurrent%20Target) 25.0 0 0)
  (Audio|PlaySoundatLocation "/Game/AIRLOCK/Sounds/minecraft_hit_sound___1080p60fps.minecraft_hit_sound___1080p60fps" (Transformation|GetActorLocation) "0, 0, 0" 1.0 1.0 0.0 0 0 0 0)
  (bind _returnvalue (Utilities|Time|SetTimerbyFunctionName 0 "Deal Contact Damage" 1.0 true))
  (Variables|Default|SetDamage%20Timer%20Handle _returnvalue))

(fn ConstructionScript)