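; First-person player character with a limited sprint meter; on player possession it adds the horror HUD widget and input mapping context.
; Sprint input or touch jump events raise walk speed and drain the meter from game-time timestamps, updating the HUD bar.
; Releasing starts a looping Recover timer that refills the meter.
; Emptying it forces a slower recovering speed, blocking sprint until the meter is full again.
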(event Custom|Sprint%20Fixed%20Tick
  ;[0.15 0.15 0.15 0.5] If we have available sprint meter & Not recovering
  (if (and (> (Variables|Sprint|GetSprint%20Meter) 0.0) (not (Variables|Recovering|GetRecovering)))
    ;[0.15 0.15 0.15 0.5] Update Time remaining on sprint meter
    (bind _output_get (Variables|Sprint|SetSprint%20Meter (- (Variables|Sprint|GetSprint%20Time%20Check) (Utilities|Time|GetGameTimeinSeconds))))
    (Default|UpdateBar (Variables|Default|GetUI_Horror) (/ _output_get (Variables|Sprint|GetSprint%20Time)))
    (else
      ;[0.15 0.15 0.15 0.5] Otherwise set recovering to true and decrease move speed
      (Variables|Recovering|SetRecovering true)
      (Variables|/Script/Engine.CharacterMovementComponent|SetMaxWalkSpeed (Variables|Character|GetCharacterMovement) (Variables|Recovering|GetRecovering%20Walk%20Speed)))))

(event Input|EnhancedActionEvents|EnhancedInputActionIA_Sprint
  (params (ActionValue :type Boolean) (ElapsedSeconds :type Float%20%28double-precision%29) (TriggeredSeconds :type Float%20%28double-precision%29) (InputAction :type Input%20Action%20Object%20Reference :default "/Game/Variant_Horror/Input/IA_Sprint.IA_Sprint"))
  (:Triggered
    ;[0.15 0.15 0.15 0.5] If we have available sprint meter & Not recovering
    (if (and (> (Variables|Sprint|GetSprint%20Meter) 0.0) (not (Variables|Recovering|GetRecovering)))
      ;[0.15 0.15 0.15 0.5] Update Time remaining on sprint meter
      (bind _output_get (Variables|Sprint|SetSprint%20Meter (- (Variables|Sprint|GetSprint%20Time%20Check) (Utilities|Time|GetGameTimeinSeconds))))
      (Default|UpdateBar (Variables|Default|GetUI_Horror) (/ _output_get (Variables|Sprint|GetSprint%20Time)))
      (else
        ;[0.15 0.15 0.15 0.5] Otherwise set recovering to true and decrease move speed
        (Variables|Recovering|SetRecovering true)
        (Variables|/Script/Engine.CharacterMovementComponent|SetMaxWalkSpeed (Variables|Character|GetCharacterMovement) (Variables|Recovering|GetRecovering%20Walk%20Speed)))))
  (:Started
    ;[0.15 0.15 0.15 0.5] If not recovering from sprint. Store Time - Current Sprint Meter & Set Sprint speed to character movement.
    (if (Variables|Recovering|GetRecovering)
      _
      (else
        (Variables|Sprint|SetSprint%20Time%20Check (+ (Utilities|Time|GetGameTimeinSeconds) (Variables|Sprint|GetSprint%20Meter)))
        (Variables|/Script/Engine.CharacterMovementComponent|SetMaxWalkSpeed (Variables|Character|GetCharacterMovement) (Variables|Sprint|GetSprint%20Speed))
        (Default|StartSprintDrain (Variables|Default|GetUI_Horror))))
    (Class|KismetSystemLibrary|PauseTimer 0 "Recover"))
  (:Canceled
    ;[0.15 0.15 0.15 0.5] Stop Sprinting and Start Recover
    (if (Variables|Recovering|GetRecovering) :!label _label
      _
      (else
        (Variables|/Script/Engine.CharacterMovementComponent|SetMaxWalkSpeed (Variables|Character|GetCharacterMovement) (Variables|Default|GetWalk%20Speed))
        (Default|StopSprintDrain (Variables|Default|GetUI_Horror))))
    (Variables|Sprint|SetSprint%20Time%20Check (- (Utilities|Time|GetGameTimeinSeconds) (Variables|Sprint|GetSprint%20Meter)))
    (Utilities|Time|SetTimerbyFunctionName 0 "Recover" 0.033333 true true))
  (:Completed
    (goto _label)))

(event EventTouchJumpStart
  (bind _returnvalue (Utilities|Time|SetTimerbyEvent (delegate Custom|Sprint%20Fixed%20Tick) 0.033333 true true))
  (Variables|Default|SetSprint%20Handle _returnvalue)
  ;[0.15 0.15 0.15 0.5] If not recovering from sprint. Store Time - Current Sprint Meter & Set Sprint speed to character movement.
  (if (Variables|Recovering|GetRecovering)
    _
    (else
      (Variables|Sprint|SetSprint%20Time%20Check (+ (Utilities|Time|GetGameTimeinSeconds) (Variables|Sprint|GetSprint%20Meter)))
      (Variables|/Script/Engine.CharacterMovementComponent|SetMaxWalkSpeed (Variables|Character|GetCharacterMovement) (Variables|Sprint|GetSprint%20Speed))
      (Default|StartSprintDrain (Variables|Default|GetUI_Horror))))
  (Class|KismetSystemLibrary|PauseTimer 0 "Recover"))

(event EventPossessed
  (params (NewController :type Controller%20Object%20Reference))
  (|CallParentFunction NewController)
  (if (Class|Controller|IsPlayerController NewController)
    ;[0.15 0.15 0.15 0.5] Create Sprint Meter UI
    (bind _asplayer_controller (Utilities|Casting|CastToPlayerController (Pawn|GetController)))
    (bind _returnvalue (UserInterface|CreateWidget "/Game/Variant_Horror/UI/UI_Horror.UI_Horror_C" _asplayer_controller))
    (bind _output_get (Variables|Default|SetUI_Horror _returnvalue))
    (UserInterface|Viewport|AddtoPlayerScreen _output_get)
    ;[0.15 0.15 0.15 0.5] Add Custom Input Mode
    (Input|AddMappingContext (PlayerController|LocalPlayerSubsystems|GetEnhancedInputLocalPlayerSubsystem _asplayer_controller) "/Game/Variant_Horror/Input/IMC_Horror.IMC_Horror" 0 "(bIgnoreAllPressedKeysUntilRelease=True,bForceImmediately=False,bNotifyUserSettings=False)")))

(event EventTouchJumpEnd
  (Utilities|Time|PauseTimerbyHandle (Variables|Default|GetSprint%20Handle))
  ;[0.15 0.15 0.15 0.5] Stop Sprinting and Start Recover
  (if (Variables|Recovering|GetRecovering)
    _
    (else
      (Variables|/Script/Engine.CharacterMovementComponent|SetMaxWalkSpeed (Variables|Character|GetCharacterMovement) (Variables|Default|GetWalk%20Speed))
      (Default|StopSprintDrain (Variables|Default|GetUI_Horror))))
  (Variables|Sprint|SetSprint%20Time%20Check (- (Utilities|Time|GetGameTimeinSeconds) (Variables|Sprint|GetSprint%20Meter)))
  (Utilities|Time|SetTimerbyFunctionName 0 "Recover" 0.033333 true true))

(fn ConstructionScript
  (|CallParentFunction))

(fn Recover
  (bind _sprint_time (Variables|Sprint|GetSprint%20Time))
  (bind _output_get (Variables|Sprint|SetSprint%20Meter (Math|Float|Min(Float) (- (Utilities|Time|GetGameTimeinSeconds) (Variables|Sprint|GetSprint%20Time%20Check)) (Variables|Sprint|GetSprint%20Time))))
  (Default|UpdateBar (Variables|Default|GetUI_Horror) (/ _output_get _sprint_time))
  (if (>= _output_get _sprint_time)
    ;[0.15 0.15 0.15 0.5] Once recovered. Return speed to normal and stop recover.
    (Class|KismetSystemLibrary|PauseTimer 0 "Recover")
    (Variables|Recovering|SetRecovering false)
    (Variables|/Script/Engine.CharacterMovementComponent|SetMaxWalkSpeed (Variables|Character|GetCharacterMovement) (Variables|Default|GetWalk%20Speed))
    (Default|StopSprintDrain (Variables|Default|GetUI_Horror))))