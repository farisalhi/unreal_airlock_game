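; Mission-end trigger volume that shows "Mission Complete" when the player arrives with three keycards.
; Every overlap adds a new WB_GameState widget to the viewport, before the BP_Player cast.
; A DoOnce precedes the keycard count check on the player's MissionWidget, so only the first player overlap is evaluated.
; On success it sets the widget text and calls DisableInput on itself with player controller 0.
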(event OnComponentBeginOverlap(Trigger)
  (params (OverlappedComponent :type Primitive%20Component%20Object%20Reference) (OtherActor :type Actor%20Object%20Reference) (OtherComp :type Primitive%20Component%20Object%20Reference) (OtherBodyIndex :type Integer) (bFromSweep :type Boolean) (SweepResult :type Hit%20Result%20Structure%20%28by%20ref%29))
  (bind _returnvalue (UserInterface|CreateWidget "/Game/AIRLOCK/UI/WB_GameState.WB_GameState_C"))
  (UserInterface|Viewport|AddtoViewport _returnvalue 0)
  (bind _asbp_player (Utilities|Casting|CastToBP_Player OtherActor))
  (Utilities|FlowControl|DoOnce false
    (:Completed
      (if (== (Variables|/Game/AIRLOCK/UI/WB_Mission.WB_Mission_C|GetKeyCards%20Collected (Variables|/Game/AIRLOCK/Blueprints/Player/BP_Player.BP_Player_C|GetMission%20Widget _asbp_player)) 3)
        (Rendering|Components|TextRender|SetText (Variables|/Game/AIRLOCK/UI/WB_GameState.WB_GameState_C|GetGameStateText _returnvalue) "Mission Complete")
        (Input|DisableInput (Game|GetPlayerController 0))))))

(event EventBeginPlay)

(event Collision|EventActorBeginOverlap
  (params (OtherActor :type Actor%20Object%20Reference)))

(event EventTick
  (params (DeltaSeconds :type Float%20%28single-precision%29)))

(fn ConstructionScript)