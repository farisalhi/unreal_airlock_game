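; BP_KeyCard is a keycard pickup that the player collects by interacting with it.
; Interact casts player 0's character to BP_Player, updates the keycard progress in its MissionWidget and makes the KeyCardContainer visible.
; It then destroys itself and, if DirectorRef is valid, calls OnKeycardCollected on it, so the director notification comes after the DestroyActor call.
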(event EventBeginPlay
  (|CallParentFunction))

(event Collision|EventActorBeginOverlap
  (params (OtherActor :type Actor%20Object%20Reference)))

(event EventTick
  (params (DeltaSeconds :type Float%20%28single-precision%29)))

(event EventInteract
  (params (Player :type BP%20Player%20Object%20Reference))
  (bind _directorref (Variables|Default|GetDirectorRef))
  (bind _asbp_player (Utilities|Casting|CastToBP_Player (Game|GetPlayerCharacter 0)))
  (Default|UpdateKeyCardProgress (Variables|/Game/AIRLOCK/Blueprints/Player/BP_Player.BP_Player_C|GetMission%20Widget _asbp_player))
  (Widget|SetVisibility (Variables|/Game/AIRLOCK/UI/WB_Mission.WB_Mission_C|GetKeyCardContainer (Variables|/Game/AIRLOCK/Blueprints/Player/BP_Player.BP_Player_C|GetMission%20Widget _asbp_player)) "Visible")
  (Actor|DestroyActor self)
  (if (Utilities|IsValid _directorref)
    (Default|OnKeycardCollected _directorref)))

(fn ConstructionScript
  (|CallParentFunction))