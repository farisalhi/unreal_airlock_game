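; BP_BaseNote is a readable note actor that the player interacts with to open a note on screen.
; Construction applies the configurable mesh and scale, and functions expose interactability and prompt name.
; Interacting with a valid DataAsset shows it in a WB_Note widget, plays a positional sound and switches to UI-only input with cursor.
; Flags optionally pause the game, save the note to the player's NoteArray or destroy the actor.
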(event EventInteract
  (params (Player :type BP%20Player%20Object%20Reference))
  ;[0.05098 0.05098 0.05098] Interact w/ Note function
  (bind _dataasset (Variables|NoteSettings|GetDataAsset)
    (:then
      (if (Variables|NoteSettings|GetPause%20Game?)
        (Game|SetGamePaused true))
      (bind _returnvalue (UserInterface|CreateWidget "/Game/FPMovement/Player/Widgets/UserCreated/Note/WB_Note.WB_Note_C" 0 _dataasset))
      (bind _output_get (Variables|Reference|SetWB%20Note _returnvalue))
      (UserInterface|Viewport|AddtoViewport _output_get 0)
      (CallFunction|PlayNoteSFX)
      (Input|SetInputModeUIOnly (Game|GetPlayerController 0) 0 "DoNotLock" false)
      (Variables|/Script/Engine.PlayerController|SetbShowMouseCursor (Game|GetPlayerController 0) true)
      (if (Variables|NoteSettings|GetSaveNote?)
        (Utilities|Array|AddUnique (Variables|/Game/FPMovement/Player/Blueprints/BP_Player.BP_Player_C|GetNoteArray Player) (Variables|NoteSettings|GetDataAsset)))
      (if (Variables|NoteSettings|GetDestroyOnRead?)
        (Utilities|IsValid self
          (:Is%20Valid
            (Actor|DestroyActor)))))
    (:else)))

(event EventBeginPlay
  ;[0.05098 0.05098 0.05098] Cast to Player
  (bind _asbp_player (Utilities|Casting|CastToBP_Player (Game|GetPlayerCharacter 0)))
  (Variables|Reference|SetPlayer%20Reference _asbp_player))

(fn ConstructionScript
  (Components|StaticMesh|SetStaticMesh (Variables|Default|GetNote) (Variables|NoteSettings|GetNote%20Mesh))
  (Transformation|SetWorldScale3D (Variables|Default|GetNote) (Math|Conversions|ToVector(Float) (Variables|NoteSettings|GetNote%20Scale))))

(fn CanInteract?
  (return (Variables|PRIVAT|GetCanInteract?)))

(event Custom|Play%20Note%20SFX
  (Audio|PlaySoundatLocation (Variables|NoteSFX|GetRead%20Note%20SFX) (Transformation|GetWorldLocation (Variables|Default|GetNote)) "0, 0, 0" (Variables|NoteSFX|GetRead%20Note%20Volume) 1.0 0.0 "/Game/FPMovement/Assets/Audio/Abilitys/Pickup/Effects/ItemAttenuation.ItemAttenuation" 0 0 0))

(fn InteractPrompt
  (return (Variables|NoteSettings|GetShow%20Note%20Prompt?) (Variables|NoteSettings|GetNote%20Name)))